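; Fluid Flux modifier component that injects force into the fluid simulation from its owning actor's movement.
; On initialization it creates a dynamic material instance, which it registers with the world as a velocity-map modifier when the world changes.
; While the owner moves, rendering passes its intensity-scaled velocity, location, radius and half height to that material and draws it onto the simulation canvas.
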(fn `ChangeWorld`
  (params (World :type "Actor Object Reference"))
  (message `/Game/FluidFlux/Simulation/Blueprints/BPI_FluxSimulationEditorCallback.UpdateModifierMaterials` World (`|MakeArray` (`self.MaterialInstance`)) true)
  (`parent.ChangeWorld` null))

(fn `InitializeModifier`
  (bind _returnvalue (`KismetMaterialLibrary.CreateDynamicMaterialInstance` (`self.Material`)))
  (set `self.MaterialInstance` _returnvalue))

(fn `RenderModifier`
  (params (Canvas :type "Canvas Object Reference") (Simulation :type "Actor Object Reference"))
  (locals (Velocity :type "Vector Structure" :default (0.0 0.0 0.0)))
  (`self.SetSimulation` Simulation)
  (set `local.Velocity` (* (`Actor.GetVelocity` (`self.GetOwner`)) (`self.Intensity`)))
  (if (> (`KismetMathLibrary.VSize` (`local.Velocity`)) 0.0)
    (`MaterialInstanceDynamic.SetVectorParameterValue` (`self.MaterialInstance`) "Velocity" (`KismetMathLibrary.Conv_VectorToLinearColor` (`local.Velocity`)))
    (`MaterialInstanceDynamic.SetVectorParameterValue` (`self.MaterialInstance`) "LocationRadius" (`KismetMathLibrary.MakeColor` (.x (.location (`Actor.GetTransform` (`self.GetOwner`)))) (.y (.location (`Actor.GetTransform` (`self.GetOwner`)))) (.z (.location (`Actor.GetTransform` (`self.GetOwner`)))) (`self.Radius`)))
    (`MaterialInstanceDynamic.SetScalarParameterValue` (`self.MaterialInstance`) "HalfHeight" (`self.HalfHeight`))
    (`Canvas.K2_DrawMaterial` (`local.Canvas`) (`self.MaterialInstance`) (0.0 0.0) (1.0 1.0) (0.0 0.0) (1.0 1.0) 0.0 (0.0 0.0))))